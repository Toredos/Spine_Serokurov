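; Enemy character that takes hits through the Gameplay Ability System and reacts with hit and death montages.
; On BeginPlay a set-by-caller effect initializes health from max health.
; ApplyHit ignores dead enemies, blends rotation to face the instigator on the horizontal plane and applies damage as a negative set-by-caller effect.
; Health changes play a hit reaction, or at zero add State.Dead, play death and disable capsule collision.
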(event EventBeginPlay
  (bind _abilitysystemcomponent (Variables|Default|GetAbilitySystemComponent))
  (bind _returnvalue (Ability|GameplayEffect|AssignTagSetbyCallerMagnitude (GameplayEffects|MakeOutgoingSpec :self _abilitysystemcomponent :GameplayEffectClass "/Game/Effects/GE_InitializeHealth.GE_InitializeHealth_C" :Level 1.0) "(TagName=\"Data.Health\")" (Class|BaseCombatCharacter|GetMaxHealth)))
  (GameplayEffects|ApplyGameplayEffectSpecToSelf _abilitysystemcomponent _returnvalue))

(event Collision|EventActorBeginOverlap
  (params (OtherActor :type Actor%20Object%20Reference)))

(event EventTick
  (params (DeltaSeconds :type Float%20%28single-precision%29)))

(event EventOnHealthChanged
  (params (OldValue :type Float%20%28single-precision%29) (NewValue :type Float%20%28single-precision%29))
  (bind _reactionplayrate (Variables|Default|GetReactionPlayRate))
  (if (<= NewValue 0.0)
    (Ability|GameplayEffect|AddLooseGameplayTags self (GameplayTags|MakeLiteralGameplayTagContainer "(GameplayTags=((TagName=\"State.Dead\")))"))
    (Animation|PlayAnimMontage "/Game/Animations/Enemy/AM_Enemy_Death.AM_Enemy_Death" _reactionplayrate "None")
    (Collision|SetCollisionEnabled (Variables|Default|GetCapsuleComponent) "NoCollision")
    (else
      (Animation|PlayAnimMontage "/Game/Animations/Enemy/AM_Enemy_HitReaction.AM_Enemy_HitReaction" _reactionplayrate "None"))))

(fn ConstructionScript)

(fn ApplyHit
  (params (Damage :type Float%20%28double-precision%29) (Instigator :type Actor%20Object%20Reference))
  (bind _returnvalue (Transformation|GetActorLocation Instigator))
  (bind _returnvalue_2 (Transformation|GetActorLocation))
  (bind _abilitysystemcomponent (Variables|Default|GetAbilitySystemComponent))
  (bind (_x _y) (Math|Vector|BreakVector _returnvalue))
  (bind (_x_2 _y_2 _z) (Math|Vector|BreakVector _returnvalue_2))
  (if (GameplayTags|HasMatchingGameplayTag _abilitysystemcomponent "(TagName=\"State.Dead\")")
    _
    (else
      (Class|BaseCombatCharacter|StartRotationBlend (Math|Rotator|FindLookatRotation (Math|Vector|MakeVector _x_2 _y_2 _z) (Math|Vector|MakeVector _x _y _z)) (Variables|Default|GetEnemyRotationBlendDuration))
      (bind _returnvalue_3 (Ability|GameplayEffect|AssignTagSetbyCallerMagnitude (GameplayEffects|MakeOutgoingSpec :self _abilitysystemcomponent :GameplayEffectClass "/Game/Effects/GE_Damage.GE_Damage_C" :Level 1.0) "(TagName=\"Data.Damage\")" (* Damage -1.0)))
      (GameplayEffects|ApplyGameplayEffectSpecToSelf _abilitysystemcomponent _returnvalue_3)))
  (return))

(fn IsAlive
  (return (not (GameplayTags|HasMatchingGameplayTag (Variables|Default|GetAbilitySystemComponent) "(TagName=\"State.Dead\")"))))