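; Gameplay ability that runs a data-driven combo attack, locking character movement and tagging the avatar as attacking until it ends.
; Each stage reads montage, damage, sounds and tag from the combo data asset, blending rotation toward movement input.
; An input press advances the combo only while the Combo.Window.Open tag is present.
; An AdvancingCombo flag distinguishes chained montage interruptions from ones that finish the combo.
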(event Custom|PlayStage
  (bind _returnvalue (Ability|GetAvatarActorfromActorInfo))
  (bind _returnvalue_2 (Ability|GetAvatarActorfromActorInfo))
  (bind _combodataasset (Variables|Default|GetComboDataAsset))
  (bind _combostageindex (Variables|Default|GetComboStageIndex))
  (bind _returnvalue_3 (Transformation|GetActorLocation _returnvalue))
  (bind _combolinks (Variables|/Game/Data/ComboAttacks/ComboAttackDataAsset.ComboAttackDataAsset_C|GetComboLinks _combodataasset))
  (bind _output (Utilities|Array|Get(acopy) _combolinks _combostageindex))
  (bind (_animmontage _activeslot _stagetag _damageamount _swingsound _hitsound) (Utilities|Struct|BreakFComboLinkData _output))
  (Ability|GameplayEffect|RemoveLooseGameplayTags _returnvalue_2 (GameplayTags|MakeGameplayTagContainerfromTag (Variables|Default|GetCurrentStageTag)))
  (bind _output_get (Variables|Default|SetCurrentStageTag _stagetag))
  (Ability|GameplayEffect|AddLooseGameplayTags _returnvalue_2 (GameplayTags|MakeGameplayTagContainerfromTag _output_get))
  (Utilities|FlowControl|Sequence
    (:then_0
      (bind _asbase_combat_character (Utilities|Casting|CastToBaseCombatCharacter (Ability|GetAvatarActorfromActorInfo)))
      (Utilities|FlowControl|Sequence
        (:then_0
          (Variables|/Script/Spine_Serokurov.BaseCombatCharacter|SetCurrentAttackDamage _asbase_combat_character _damageamount)
          (Class|BaseCombatCharacter|DisableAllWeaponCollisionSlots _asbase_combat_character)
          (bind _asbase_combat_character_2 (Utilities|Casting|CastToBaseCombatCharacter (Ability|GetAvatarActorfromActorInfo))
            (:then
              (if (> (Math|Vector|VectorLength (Class|BaseCombatCharacter|GetCurrentMovementInputDirection _asbase_combat_character_2)) 0.1)
                (bind _asbase_combat_character_3 (Utilities|Casting|CastToBaseCombatCharacter _returnvalue)
                  (:then
                    (Class|BaseCombatCharacter|StartRotationBlend _asbase_combat_character_3 (Math|Rotator|FindLookatRotation _returnvalue_3 (+ _returnvalue_3 (Class|BaseCombatCharacter|GetCurrentMovementInputDirection _asbase_combat_character_2))) (Variables|Default|GetRotationBlendDuration)))
                  (:CastFailed
                    _))))
            (:CastFailed
              _))
          (|PlayMontageandWaitProxy "None" _animmontage (Variables|Default|GetAttackPlayRate) "None" true 1.0 0.0 false
            (:OnCompleted
              (CallFunction|FinishCombo :!label _label))
            (:OnInterrupted
              (if (Variables|Default|GetbAdvancingCombo)
                (Variables|Default|SetbAdvancingCombo false)
                (else
                  (goto _label))))
            (:OnCancelled
              (goto _label))))
        (:then_1
          (Audio|PlaySound2D _swingsound 1.0 1.0 0.0 0 0))
        (:then_2
          (Variables|/Script/Spine_Serokurov.BaseCombatCharacter|SetCurrentAttackHitSound _asbase_combat_character _hitsound))))
    (:then_1
      (CallFunction|ListenforInput))))

(event Custom|ListenForInput
  (Ability|Tasks|WaitInputPress false
    (:OnPress
      (if (and (GameplayTags|HasMatchingGameplayTag (Ability|GetAbilitySystemComponentfromActorInfo) "(TagName=\"Combo.Window.Open\")") (< (Variables|Default|GetComboStageIndex) (- (Utilities|Array|Length (Variables|/Game/Data/ComboAttacks/ComboAttackDataAsset.ComboAttackDataAsset_C|GetComboLinks (Variables|Default|GetComboDataAsset))) 1)))
        (Variables|Default|SetbAdvancingCombo true)
        (Variables|Default|SetComboStageIndex (+ (Variables|Default|GetComboStageIndex) 1))
        (CallFunction|PlayStage)
        (elif (Math|Conversions|ToBoolean(Integer) (+ (Variables|Default|GetComboStageIndex) 1))
          (CallFunction|ListenforInput))))))

(event Ability|EventActivateAbility
  (bind _returnvalue (Ability|GetAvatarActorfromActorInfo))
  (bind _ascharacter (Utilities|Casting|CastToCharacter _returnvalue)
    (:then
      (Variables|Default|SetOriginalMaxWalkSpeed (Variables|/Script/Engine.CharacterMovementComponent|GetMaxWalkSpeed (Variables|/Script/Engine.Character|GetCharacterMovement _ascharacter)))
      (Variables|/Script/Engine.CharacterMovementComponent|SetMaxWalkSpeed (Variables|/Script/Engine.Character|GetCharacterMovement _ascharacter) 0.0)
      (Variables|/Script/Engine.CharacterMovementComponent|SetbOrientRotationToMovement (Variables|/Script/Engine.Character|GetCharacterMovement _ascharacter) false)
      (Components|Movement|StopMovementImmediately (Variables|/Script/Engine.Character|GetCharacterMovement _ascharacter)))
    (:CastFailed
      _))
  (bind _returnvalue_2 (Ability|CommitAbility))
  (if _returnvalue_2
    (Variables|Default|SetComboStageIndex 0)
    (Ability|GameplayEffect|AddLooseGameplayTags _returnvalue (GameplayTags|MakeLiteralGameplayTagContainer "(GameplayTags=((TagName=\"State.Attacking\")))"))
    (CallFunction|PlayStage)
    (else
      (Ability|CancelAbility))))

(event Ability|EventOnEndAbility
  (params (bWasCancelled :type Boolean))
  (bind _returnvalue (Ability|GetAvatarActorfromActorInfo))
  (bind _ascharacter (Utilities|Casting|CastToCharacter _returnvalue)
    (:then
      _)
    (:CastFailed
      _))
  (Utilities|FlowControl|Sequence
    (:then_0
      (Variables|/Script/Engine.CharacterMovementComponent|SetMaxWalkSpeed (Variables|/Script/Engine.Character|GetCharacterMovement _ascharacter) (Variables|Default|GetOriginalMaxWalkSpeed)))
    (:then_1
      (Variables|/Script/Engine.CharacterMovementComponent|SetbOrientRotationToMovement (Variables|/Script/Engine.Character|GetCharacterMovement _ascharacter) true))
    (:then_2
      (Ability|GameplayEffect|RemoveLooseGameplayTags _returnvalue (GameplayTags|MakeLiteralGameplayTagContainer "(GameplayTags=((TagName=\"State.Attacking\")))")))))

(fn FinishCombo
  (bind _returnvalue (Ability|GetAvatarActorfromActorInfo))
  (Ability|GameplayEffect|RemoveLooseGameplayTags _returnvalue (GameplayTags|MakeLiteralGameplayTagContainer "(GameplayTags=((TagName=\"State.Attacking\")))"))
  (Ability|GameplayEffect|RemoveLooseGameplayTags _returnvalue (GameplayTags|MakeGameplayTagContainerfromTag (Variables|Default|GetCurrentStageTag)))
  (Variables|Default|SetComboStageIndex 0)
  (Ability|EndAbility))