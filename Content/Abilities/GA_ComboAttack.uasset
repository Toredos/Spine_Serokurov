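; Combo attack gameplay ability, apparently unfinished: activation commits, resets the stage index and adds a local State.Attacking tag, or cancels.
; PlayStage swaps stage A/B/C tags by index, plays that link's data-asset montage and waits for input, with neither task's result handled.
; Its only call is disconnected.
; FinishCombo clears only the stage A tag, resets the index and ends the ability, leaving State.Attacking in place.
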(event Custom|PlayStage
  (bind _returnvalue (GameplayTags|MakeLiteralGameplayTagContainer "(GameplayTags=((TagName=\"Combo.Stage.B\")))"))
  (bind _returnvalue_2 (Ability|GetAvatarActorfromActorInfo))
  (bind _returnvalue_3 (GameplayTags|MakeLiteralGameplayTagContainer "(GameplayTags=((TagName=\"Combo.Stage.C\")))"))
  (bind _returnvalue_4 (GameplayTags|MakeLiteralGameplayTagContainer "(GameplayTags=((TagName=\"Combo.Stage.A\")))"))
  (bind _combostageindex (Variables|Default|GetComboStageIndex))
  (Ability|GameplayEffect|RemoveLooseGameplayTags _returnvalue_2 _returnvalue_4)
  (Ability|GameplayEffect|RemoveLooseGameplayTags _returnvalue_2 _returnvalue)
  (Ability|GameplayEffect|RemoveLooseGameplayTags _returnvalue_2 _returnvalue_3)
  (switch int _combostageindex
    (:0
      (Ability|GameplayEffect|AddLooseGameplayTags _returnvalue_2 _returnvalue_4))
    (:1
      (Ability|GameplayEffect|AddLooseGameplayTags _returnvalue_2 _returnvalue))
    (:2
      (Ability|GameplayEffect|AddLooseGameplayTags _returnvalue_2 _returnvalue_3)))
  (Utilities|FlowControl|Sequence
    (:then_0
      (|PlayMontageandWaitProxy "None" (.AnimMontage (Utilities|Struct|BreakFComboLinkData (Utilities|Array|Get(acopy) (Variables|/Game/Data/ComboAttackDataAsset.ComboAttackDataAsset_C|GetComboLinks (Variables|Default|GetComboDataAsset)) _combostageindex))) 1.0 "None" true 1.0 0.0 false))
    (:then_1
      (Ability|Tasks|WaitInputPress false))))

(event Ability|EventActivateAbility
  (bind _returnvalue (Ability|CommitAbility))
  (if _returnvalue
    (Variables|Default|SetComboStageIndex 0)
    (Ability|GameplayEffect|AddLooseGameplayTags (Ability|GetAvatarActorfromActorInfo) (GameplayTags|MakeLiteralGameplayTagContainer "(GameplayTags=((TagName=\"State.Attacking\")))"))
    (else
      (Ability|CancelAbility))))

(event Ability|EventOnEndAbility
  (params (bWasCancelled :type Boolean)))

(fn FinishCombo
  (Ability|GameplayEffect|RemoveLooseGameplayTags (Ability|GetAvatarActorfromActorInfo) (GameplayTags|MakeLiteralGameplayTagContainer "(GameplayTags=((TagName=\"Combo.Stage.A\"),(TagName=\"Combo.Stage.B\"),(TagName=\"Combo.Stage.C\"),(TagName=\"State.Attacking\")))"))
  (Variables|Default|SetComboStageIndex 0)
  (Ability|EndAbility))